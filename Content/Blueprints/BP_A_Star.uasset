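; A* pathfinder that returns a tile path between two points on a grid, with optional diagonal moves.
; FindPath expands the cheapest discovered tile, kept in cost-sorted parallel arrays, and stops once the target is discovered.
; Every step costs 1; grid tile types only add penalties to the Manhattan or Chebyshev estimate.
; Neighbors are not bounds-checked; the path is rebuilt from previous-tile links, excluding the start.
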(event EventBeginPlay)

(event Collision|EventActorBeginOverlap
  (params (OtherActor :type Actor%20Object%20Reference)))

(event EventTick
  (params (DeltaSeconds :type Float%20%28single-precision%29)))

(fn ConstructionScript)

(fn FindPath
  (params (Start :type Int%20Point%20Structure) (Target :type Int%20Point%20Structure) (Diagonals :type Boolean) (grid :type Map%20of%20Vector%202D%20Structures%20to%20Bytes))
  (Variables|Default|SetStart Start)
  (Variables|Default|SetTarget Target)
  (Variables|Default|SetDiagonals Diagonals)
  (Variables|Default|SetGrid grid)
  (CallFunction|ClearGeneratedData)
  (bind _isvalid (CallFunction|IsInputDataValid))
  (if _isvalid
    (CallFunction|DiscoverTile (Utilities|Struct|MakeS_PathFindingData (Variables|Default|GetStart) 1 0 (CallFunction|GetMinimunCostBetweenTwoTiles (Variables|Default|GetStart) (Variables|Default|GetTarget) (Variables|Default|GetDiagonals)) "(X=-999,Y=999)"))
    (while (> (Utilities|Array|Length (Variables|Default|GetDiscoveredTilesIndexes)) 0)
      (bind _foundtargettile (CallFunction|AnalizeNextDiscoveredTile))
      (if _foundtargettile
        (bind _path (CallFunction|GeneratePath))
        (return _path)))
    (return (Utilities|Array|MakeArray))
    (else
      (return (Utilities|Array|MakeArray)))))

(fn IsInputDataValid
  (if (!= (Variables|Default|GetStart) (Variables|Default|GetTarget))
    (return true)
    (else
      (return false))))

(fn DiscoverTile
  (params (TilePathData :type S%20Path%20Finding%20Data%20Structure))
  (Utilities|Map|Add (Variables|Default|GetPathFindingData) (.Index (Utilities|Struct|BreakS_PathFindingData TilePathData)) TilePathData)
  (CallFunction|InsertTileinDiscoveredArray TilePathData))

(fn GetMinimunCostBetweenTwoTiles
  (params (Index1 :type Int%20Point%20Structure) (Index2 :type Int%20Point%20Structure) (Diagonals :type Boolean))
  (bind _grid (Variables|Default|GetGrid))
  (bind _returnvalue (Math|Conversions|ToVector2D(IntPoint) Index2))
  (bind _returnvalue_2 (- Index1 Index2))
  (bind _returnvalue_3 (- Index1 Index2))
  (bind _value (Utilities|Map|Find _grid _returnvalue))
  (if Diagonals
    (LocalVariables|Setcost (Math|Integer|Max(Integer) (Math|Integer|Absolute(Integer) (.x _returnvalue_3)) (Math|Integer|Absolute(Integer) (.y _returnvalue_3))))
    (else
      (LocalVariables|Setcost (+ (Math|Integer|Absolute(Integer) (.x _returnvalue_2)) (Math|Integer|Absolute(Integer) (.y _returnvalue_2))))))
  (if (Utilities|Enum|Equal(Enum) _value "NewEnumerator1")
    (LocalVariables|Setcost (+ (LocalVariables|Getcost) 10))
    (return (LocalVariables|Getcost))
    (elif (Utilities|Enum|Equal(Enum) _value "NewEnumerator0")
      (LocalVariables|Setcost (+ (LocalVariables|Getcost) 5))
      (return (LocalVariables|Getcost))
      (elif (Utilities|Enum|Equal(Enum) _value "NewEnumerator2")
        (LocalVariables|Setcost (+ (LocalVariables|Getcost) 1))
        (return (LocalVariables|Getcost))
        (else
          (return (LocalVariables|Getcost)))))))

(fn AnalizeNextDiscoveredTile
  (bind _tilepathdta (CallFunction|PullCheapestTileOutOfDiscoveredList))
  (Variables|Default|SetCurrentDiscovedTile _tilepathdta)
  (bind _neighbors (CallFunction|GetValidTileNeighbors (.Index (Utilities|Struct|BreakS_PathFindingData (Variables|Default|GetCurrentDiscovedTile))) (Variables|Default|GetDiagonals)))
  (Variables|Default|SetCurrentNeighbors _neighbors)
  (while (> (Utilities|Array|Length (Variables|Default|GetCurrentNeighbors)) 0)
    (bind _istargettile (CallFunction|DiscoverNextNeighbor))
    (if _istargettile
      (return true)))
  (return false))

(fn GeneratePath
  (LocalVariables|SetCurrent (Variables|Default|GetTarget))
  (while (!= (LocalVariables|GetCurrent) (Variables|Default|GetStart))
    (Utilities|Array|Add (LocalVariables|GetInvertedPath) (LocalVariables|GetCurrent))
    (LocalVariables|SetCurrent (.PreviousIndex (Utilities|Struct|BreakS_PathFindingData (.Value (Utilities|Map|Find (Variables|Default|GetPathFindingData) (LocalVariables|GetCurrent)))))))
  (bind _arrayelement (Utilities|Array|ReverseforEachLoop (LocalVariables|GetInvertedPath))
    (:LoopBody
      (Utilities|Array|Add (LocalVariables|GetReversed) _arrayelement))
    (:Completed
      (return (LocalVariables|GetReversed)))))

(fn PullCheapestTileOutOfDiscoveredList
  (LocalVariables|SetTileIndex (Utilities|Array|Get(acopy) (Variables|Default|GetDiscoveredTilesIndexes)))
  (Utilities|Array|RemoveIndex (Variables|Default|GetDiscoveredTilesSortingCost))
  (Utilities|Array|RemoveIndex (Variables|Default|GetDiscoveredTilesIndexes))
  (Utilities|Array|Add (Variables|Default|GetAnalisedTileIndexes) (LocalVariables|GetTileIndex))
  (return (.Value (Utilities|Map|Find (Variables|Default|GetPathFindingData) (LocalVariables|GetTileIndex)))))

(fn GetValidTileNeighbors
  (params (Tile :type Int%20Point%20Structure) (Diagonals :type Boolean))
  (bind _response (LocalVariables|Getresponse))
  (bind _response_2 (LocalVariables|Getresponse))
  (Utilities|Array|Clear (LocalVariables|Getresponse))
  (LocalVariables|SetI_Tile Tile)
  (LocalVariables|SetI_Diagonals Diagonals)
  (Utilities|Array|Add _response_2 (Utilities|Struct|MakeS_PathFindingData (- (LocalVariables|GetI_Tile) (Utilities|Struct|MakeIntPoint 0 1)) 1))
  (Utilities|Array|Add _response_2 (Utilities|Struct|MakeS_PathFindingData (+ (LocalVariables|GetI_Tile) (Utilities|Struct|MakeIntPoint 1 0)) 1))
  (Utilities|Array|Add _response_2 (Utilities|Struct|MakeS_PathFindingData (+ (LocalVariables|GetI_Tile) (Utilities|Struct|MakeIntPoint 0 1)) 1))
  (Utilities|Array|Add _response_2 (Utilities|Struct|MakeS_PathFindingData (- (LocalVariables|GetI_Tile) (Utilities|Struct|MakeIntPoint 1 0)) 1))
  (if (LocalVariables|GetI_Diagonals)
    (Utilities|Array|Add _response (Utilities|Struct|MakeS_PathFindingData (+ (LocalVariables|GetI_Tile) (Utilities|Struct|MakeIntPoint -1 -1)) 1))
    (Utilities|Array|Add _response (Utilities|Struct|MakeS_PathFindingData (+ (LocalVariables|GetI_Tile) (Utilities|Struct|MakeIntPoint 1 -1)) 1))
    (Utilities|Array|Add _response (Utilities|Struct|MakeS_PathFindingData (+ (LocalVariables|GetI_Tile) (Utilities|Struct|MakeIntPoint 1 1)) 1))
    (Utilities|Array|Add _response (Utilities|Struct|MakeS_PathFindingData (+ (LocalVariables|GetI_Tile) (Utilities|Struct|MakeIntPoint -1 1)) 1))
    (return (LocalVariables|Getresponse))
    (else
      (return (LocalVariables|Getresponse)))))

(fn DiscoverNextNeighbor
  (Variables|Default|SetCurrentNeighbor (Utilities|Array|Get(acopy) (Variables|Default|GetCurrentNeighbors)))
  (Utilities|Array|RemoveIndex (Variables|Default|GetCurrentNeighbors))
  (if (not (Utilities|Array|ContainsItem (Variables|Default|GetAnalisedTileIndexes) (.Index (Utilities|Struct|BreakS_PathFindingData (Variables|Default|GetCurrentNeighbor)))))
    (LocalVariables|SetCostFromStart (+ (.CostFromStart (Utilities|Struct|BreakS_PathFindingData (Variables|Default|GetCurrentDiscovedTile))) (.CostToEnterTile (Utilities|Struct|BreakS_PathFindingData (Variables|Default|GetCurrentNeighbor)))))
    (bind _output_get (LocalVariables|SetIndexInDiscovered (Utilities|Array|FindItem (Variables|Default|GetDiscoveredTilesIndexes) (.Index (Utilities|Struct|BreakS_PathFindingData (Variables|Default|GetCurrentNeighbor))))))
    (if (== _output_get -1)
      _
      (else
        (bind _output_get_2 (Variables|Default|SetCurrentNeighbor (.Value (Utilities|Map|Find (Variables|Default|GetPathFindingData) (.Index (Utilities|Struct|BreakS_PathFindingData (Variables|Default|GetCurrentNeighbor)))))))
        (if (< (LocalVariables|GetCostFromStart) (.CostFromStart (Utilities|Struct|BreakS_PathFindingData _output_get_2)))
          (Utilities|Array|RemoveIndex (Variables|Default|GetDiscoveredTilesIndexes) (LocalVariables|GetIndexInDiscovered))
          (Utilities|Array|RemoveIndex (Variables|Default|GetDiscoveredTilesSortingCost) (LocalVariables|GetIndexInDiscovered))
          (else
            (return false)))))
    (CallFunction|DiscoverTile (Utilities|Struct|MakeS_PathFindingData (.Index (Utilities|Struct|BreakS_PathFindingData (Variables|Default|GetCurrentNeighbor))) (.CostToEnterTile (Utilities|Struct|BreakS_PathFindingData (Variables|Default|GetCurrentNeighbor))) (LocalVariables|GetCostFromStart) (CallFunction|GetMinimunCostBetweenTwoTiles (.Index (Utilities|Struct|BreakS_PathFindingData (Variables|Default|GetCurrentNeighbor))) (Variables|Default|GetTarget) (Variables|Default|GetDiagonals)) (.Index (Utilities|Struct|BreakS_PathFindingData (Variables|Default|GetCurrentDiscovedTile)))))
    (if (Class|KismetMathLibrary|EqualIntPointIntPoint (.Index (Utilities|Struct|BreakS_PathFindingData (Variables|Default|GetCurrentNeighbor))) (Variables|Default|GetTarget))
      (return true)
      (else
        (return false)))
    (else
      (return false))))

(fn InsertTileinDiscoveredArray
  (params (TileData :type S%20Path%20Finding%20Data%20Structure))
  (bind (_index _costtoentertile _costfromstart _minimuncosttotarget) (Utilities|Struct|BreakS_PathFindingData TileData))
  (bind _discoveredtilessortingcost (Variables|Default|GetDiscoveredTilesSortingCost))
  (LocalVariables|SetSortingCost (+ _costfromstart _minimuncosttotarget))
  (if (== (Utilities|Array|Length (Variables|Default|GetDiscoveredTilesSortingCost)) 0)
    (Utilities|Array|Add (Variables|Default|GetDiscoveredTilesSortingCost) (LocalVariables|GetSortingCost) :!label _label)
    (Utilities|Array|Add (Variables|Default|GetDiscoveredTilesIndexes) (.Index (Utilities|Struct|BreakS_PathFindingData TileData)))
    (elif (>= (LocalVariables|GetSortingCost) (Utilities|Array|Get(acopy) _discoveredtilessortingcost (Utilities|Array|LastIndex _discoveredtilessortingcost)))
      (goto _label)
      (else
        (bind (_array_element _array_index) (Utilities|Array|ForEachLoopwithBreak (Variables|Default|GetDiscoveredTilesSortingCost) :!label _label_2)
          (:LoopBody
            (if (>= _array_element (LocalVariables|GetSortingCost))
              (Utilities|Array|Insert (Variables|Default|GetDiscoveredTilesSortingCost) (LocalVariables|GetSortingCost) _array_index)
              (Utilities|Array|Insert (Variables|Default|GetDiscoveredTilesIndexes) (.Index (Utilities|Struct|BreakS_PathFindingData TileData)) _array_index)
              (goto _label_2 Break))))))))

(fn ClearGeneratedData
  (Utilities|Map|Clear (Variables|Default|GetPathFindingData))
  (Utilities|Array|Clear (Variables|Default|GetDiscoveredTilesSortingCost))
  (Utilities|Array|Clear (Variables|Default|GetDiscoveredTilesIndexes))
  (Utilities|Array|Clear (Variables|Default|GetAnalisedTileIndexes)))