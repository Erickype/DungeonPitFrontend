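; Actor that builds a dungeon section from a layout generated by a gRPC DungeonService, requested through TurboLink on BeginPlay.
; The response's typed grid lines are scaled by Offset and drawn as color-coded debug lines.
; Room and hallway lines become IEMWall instances at segment midpoints, and doors get IEMArch instances at both ends, all rotated by horizontal or vertical orientation.
; Hallway paths are debug-only, and failed responses are logged.
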(event Custom|OnGenerateDungeonResponse
  (params (Handle :type Grpc%20Context%20Handle%20Structure) (GrpcResult :type Grpc%20Result%20Structure%20%28by%20ref%29) (Response :type Grpc%20Dungeon%20Generate%20Dungeon%20Response%20Structure%20%28by%20ref%29))
  (bind _iemarch (Variables|Default|GetIEMArch))
  (bind _iemarch_2 (Variables|Default|GetIEMArch))
  (if (Utilities|Enum|Equal(Enum) (.code GrpcResult) "Ok")
    (bind _output_get (Variables|Default|SetGridLines (Utilities|Struct|BreakGrpcDungeonGenerateDungeonResponse Response)))
    (for _array_element _output_get
      (switch Utilities|FlowControl|Switch|SwitchonE_LineType (Utilities|Enum|ByteToEnumE_LineType (Math|Conversions|ToByte(Integer) (Class|KismetMathLibrary|ToInt64(Byte) (.linetype _array_element))))
        (:NewEnumerator0
          (Rendering|Debug|DrawDebugLine (Math|Conversions|ToVector(Vector2D) (* (.A (Utilities|Struct|BreakLine (Utilities|Struct|MakeLine (Math|Vector2D|MakeVector2D (Math|Conversions|ToFloat(Integer) (.x (.a (.line _array_element)))) (Math|Conversions|ToFloat(Integer) (.y (.a (.line _array_element))))) (Math|Vector2D|MakeVector2D (Math|Conversions|ToFloat(Integer) (.x (.b (.line _array_element)))) (Math|Conversions|ToFloat(Integer) (.y (.b (.line _array_element)))))))) (Variables|Default|Getoffset2DVector)) (Variables|Default|GetOffset%20Z)) (Math|Conversions|ToVector(Vector2D) (* (.B (Utilities|Struct|BreakLine (Utilities|Struct|MakeLine (Math|Vector2D|MakeVector2D (Math|Conversions|ToFloat(Integer) (.x (.a (.line _array_element)))) (Math|Conversions|ToFloat(Integer) (.y (.a (.line _array_element))))) (Math|Vector2D|MakeVector2D (Math|Conversions|ToFloat(Integer) (.x (.b (.line _array_element)))) (Math|Conversions|ToFloat(Integer) (.y (.b (.line _array_element)))))))) (Variables|Default|Getoffset2DVector)) (Variables|Default|GetOffset%20Z)) "(R=0.061461,G=1.000000,B=0.025231,A=1.000000)" 5e+03 3.0)
          (bind _horizontal (CallFunction|GetOrientationfromTwoPoints (Class|KismetMathLibrary|ToIntPoint(Vector2D) (* (.A (Utilities|Struct|BreakLine (Utilities|Struct|MakeLine (Math|Vector2D|MakeVector2D (Math|Conversions|ToFloat(Integer) (.x (.a (.line _array_element)))) (Math|Conversions|ToFloat(Integer) (.y (.a (.line _array_element))))) (Math|Vector2D|MakeVector2D (Math|Conversions|ToFloat(Integer) (.x (.b (.line _array_element)))) (Math|Conversions|ToFloat(Integer) (.y (.b (.line _array_element)))))))) (Variables|Default|Getoffset2DVector))) (Class|KismetMathLibrary|ToIntPoint(Vector2D) (* (.B (Utilities|Struct|BreakLine (Utilities|Struct|MakeLine (Math|Vector2D|MakeVector2D (Math|Conversions|ToFloat(Integer) (.x (.a (.line _array_element)))) (Math|Conversions|ToFloat(Integer) (.y (.a (.line _array_element))))) (Math|Vector2D|MakeVector2D (Math|Conversions|ToFloat(Integer) (.x (.b (.line _array_element)))) (Math|Conversions|ToFloat(Integer) (.y (.b (.line _array_element)))))))) (Variables|Default|Getoffset2DVector)))))
          (switch Utilities|FlowControl|Switch|SwitchonE_Orientation _horizontal
            (:NewEnumerator0
              (Components|InstancedStaticMesh|AddInstance (Variables|Default|GetIEMWall) (Math|Transform|MakeTransform (Math|Vector|MakeVector (+ (.X (Math|Vector2D|BreakVector2D (* (.A (Utilities|Struct|BreakLine (Utilities|Struct|MakeLine (Math|Vector2D|MakeVector2D (Math|Conversions|ToFloat(Integer) (.x (.a (.line _array_element)))) (Math|Conversions|ToFloat(Integer) (.y (.a (.line _array_element))))) (Math|Vector2D|MakeVector2D (Math|Conversions|ToFloat(Integer) (.x (.b (.line _array_element)))) (Math|Conversions|ToFloat(Integer) (.y (.b (.line _array_element)))))))) (Variables|Default|Getoffset2DVector)))) (/ (Math|Vector|Distance2D(Vector) (* (.A (Utilities|Struct|BreakLine (Utilities|Struct|MakeLine (Math|Vector2D|MakeVector2D (Math|Conversions|ToFloat(Integer) (.x (.a (.line _array_element)))) (Math|Conversions|ToFloat(Integer) (.y (.a (.line _array_element))))) (Math|Vector2D|MakeVector2D (Math|Conversions|ToFloat(Integer) (.x (.b (.line _array_element)))) (Math|Conversions|ToFloat(Integer) (.y (.b (.line _array_element)))))))) (Variables|Default|Getoffset2DVector)) (* (.B (Utilities|Struct|BreakLine (Utilities|Struct|MakeLine (Math|Vector2D|MakeVector2D (Math|Conversions|ToFloat(Integer) (.x (.a (.line _array_element)))) (Math|Conversions|ToFloat(Integer) (.y (.a (.line _array_element))))) (Math|Vector2D|MakeVector2D (Math|Conversions|ToFloat(Integer) (.x (.b (.line _array_element)))) (Math|Conversions|ToFloat(Integer) (.y (.b (.line _array_element)))))))) (Variables|Default|Getoffset2DVector))) 2.0)) (.Y (Math|Vector2D|BreakVector2D (* (.A (Utilities|Struct|BreakLine (Utilities|Struct|MakeLine (Math|Vector2D|MakeVector2D (Math|Conversions|ToFloat(Integer) (.x (.a (.line _array_element)))) (Math|Conversions|ToFloat(Integer) (.y (.a (.line _array_element))))) (Math|Vector2D|MakeVector2D (Math|Conversions|ToFloat(Integer) (.x (.b (.line _array_element)))) (Math|Conversions|ToFloat(Integer) (.y (.b (.line _array_element)))))))) (Variables|Default|Getoffset2DVector)))) 0.0) "0, 0, 0" "0.750000,0.750000,1.000000") true))
            (:NewEnumerator1
              (Components|InstancedStaticMesh|AddInstance (Variables|Default|GetIEMWall) (Math|Transform|MakeTransform (Math|Vector|MakeVector (.X (Math|Vector2D|BreakVector2D (* (.A (Utilities|Struct|BreakLine (Utilities|Struct|MakeLine (Math|Vector2D|MakeVector2D (Math|Conversions|ToFloat(Integer) (.x (.a (.line _array_element)))) (Math|Conversions|ToFloat(Integer) (.y (.a (.line _array_element))))) (Math|Vector2D|MakeVector2D (Math|Conversions|ToFloat(Integer) (.x (.b (.line _array_element)))) (Math|Conversions|ToFloat(Integer) (.y (.b (.line _array_element)))))))) (Variables|Default|Getoffset2DVector)))) (+ (.Y (Math|Vector2D|BreakVector2D (* (.A (Utilities|Struct|BreakLine (Utilities|Struct|MakeLine (Math|Vector2D|MakeVector2D (Math|Conversions|ToFloat(Integer) (.x (.a (.line _array_element)))) (Math|Conversions|ToFloat(Integer) (.y (.a (.line _array_element))))) (Math|Vector2D|MakeVector2D (Math|Conversions|ToFloat(Integer) (.x (.b (.line _array_element)))) (Math|Conversions|ToFloat(Integer) (.y (.b (.line _array_element)))))))) (Variables|Default|Getoffset2DVector)))) (/ (Math|Vector|Distance2D(Vector) (* (.A (Utilities|Struct|BreakLine (Utilities|Struct|MakeLine (Math|Vector2D|MakeVector2D (Math|Conversions|ToFloat(Integer) (.x (.a (.line _array_element)))) (Math|Conversions|ToFloat(Integer) (.y (.a (.line _array_element))))) (Math|Vector2D|MakeVector2D (Math|Conversions|ToFloat(Integer) (.x (.b (.line _array_element)))) (Math|Conversions|ToFloat(Integer) (.y (.b (.line _array_element)))))))) (Variables|Default|Getoffset2DVector)) (* (.B (Utilities|Struct|BreakLine (Utilities|Struct|MakeLine (Math|Vector2D|MakeVector2D (Math|Conversions|ToFloat(Integer) (.x (.a (.line _array_element)))) (Math|Conversions|ToFloat(Integer) (.y (.a (.line _array_element))))) (Math|Vector2D|MakeVector2D (Math|Conversions|ToFloat(Integer) (.x (.b (.line _array_element)))) (Math|Conversions|ToFloat(Integer) (.y (.b (.line _array_element)))))))) (Variables|Default|Getoffset2DVector))) 2.0)) 0.0) "0.000000,90.000000,0.000000" "0.750000,0.750000,1.000000") true))))
        (:NewEnumerator4
          (Rendering|Debug|DrawDebugLine (Math|Conversions|ToVector(Vector2D) (* (.A (Utilities|Struct|BreakLine (Utilities|Struct|MakeLine (Math|Vector2D|MakeVector2D (Math|Conversions|ToFloat(Integer) (.x (.a (.line _array_element)))) (Math|Conversions|ToFloat(Integer) (.y (.a (.line _array_element))))) (Math|Vector2D|MakeVector2D (Math|Conversions|ToFloat(Integer) (.x (.b (.line _array_element)))) (Math|Conversions|ToFloat(Integer) (.y (.b (.line _array_element)))))))) (Variables|Default|Getoffset2DVector)) (Variables|Default|GetOffset%20Z)) (Math|Conversions|ToVector(Vector2D) (* (.B (Utilities|Struct|BreakLine (Utilities|Struct|MakeLine (Math|Vector2D|MakeVector2D (Math|Conversions|ToFloat(Integer) (.x (.a (.line _array_element)))) (Math|Conversions|ToFloat(Integer) (.y (.a (.line _array_element))))) (Math|Vector2D|MakeVector2D (Math|Conversions|ToFloat(Integer) (.x (.b (.line _array_element)))) (Math|Conversions|ToFloat(Integer) (.y (.b (.line _array_element)))))))) (Variables|Default|Getoffset2DVector)) (Variables|Default|GetOffset%20Z)) "(R=0.827448,G=1.000000,B=0.000000,A=1.000000)" 5e+03 3.0)
          (bind _horizontal_2 (CallFunction|GetOrientationfromTwoPoints (Class|KismetMathLibrary|ToIntPoint(Vector2D) (* (.A (Utilities|Struct|BreakLine (Utilities|Struct|MakeLine (Math|Vector2D|MakeVector2D (Math|Conversions|ToFloat(Integer) (.x (.a (.line _array_element)))) (Math|Conversions|ToFloat(Integer) (.y (.a (.line _array_element))))) (Math|Vector2D|MakeVector2D (Math|Conversions|ToFloat(Integer) (.x (.b (.line _array_element)))) (Math|Conversions|ToFloat(Integer) (.y (.b (.line _array_element)))))))) (Variables|Default|Getoffset2DVector))) (Class|KismetMathLibrary|ToIntPoint(Vector2D) (* (.B (Utilities|Struct|BreakLine (Utilities|Struct|MakeLine (Math|Vector2D|MakeVector2D (Math|Conversions|ToFloat(Integer) (.x (.a (.line _array_element)))) (Math|Conversions|ToFloat(Integer) (.y (.a (.line _array_element))))) (Math|Vector2D|MakeVector2D (Math|Conversions|ToFloat(Integer) (.x (.b (.line _array_element)))) (Math|Conversions|ToFloat(Integer) (.y (.b (.line _array_element)))))))) (Variables|Default|Getoffset2DVector)))))
          (switch Utilities|FlowControl|Switch|SwitchonE_Orientation _horizontal_2
            (:NewEnumerator0
              (Components|InstancedStaticMesh|AddInstance _iemarch_2 (Math|Transform|MakeTransform (Math|Conversions|ToVector(Vector2D) (* (.A (Utilities|Struct|BreakLine (Utilities|Struct|MakeLine (Math|Vector2D|MakeVector2D (Math|Conversions|ToFloat(Integer) (.x (.a (.line _array_element)))) (Math|Conversions|ToFloat(Integer) (.y (.a (.line _array_element))))) (Math|Vector2D|MakeVector2D (Math|Conversions|ToFloat(Integer) (.x (.b (.line _array_element)))) (Math|Conversions|ToFloat(Integer) (.y (.b (.line _array_element)))))))) (Variables|Default|Getoffset2DVector))) "0, 0, 0" "1.200000,1.000000,1.000000") true)
              (Components|InstancedStaticMesh|AddInstance _iemarch_2 (Math|Transform|MakeTransform (Math|Conversions|ToVector(Vector2D) (* (.B (Utilities|Struct|BreakLine (Utilities|Struct|MakeLine (Math|Vector2D|MakeVector2D (Math|Conversions|ToFloat(Integer) (.x (.a (.line _array_element)))) (Math|Conversions|ToFloat(Integer) (.y (.a (.line _array_element))))) (Math|Vector2D|MakeVector2D (Math|Conversions|ToFloat(Integer) (.x (.b (.line _array_element)))) (Math|Conversions|ToFloat(Integer) (.y (.b (.line _array_element)))))))) (Variables|Default|Getoffset2DVector))) "0.000000,180.000000,0.000000" "1.200000,1.000000,1.000000") true))
            (:NewEnumerator1
              (Components|InstancedStaticMesh|AddInstance _iemarch (Math|Transform|MakeTransform (Math|Conversions|ToVector(Vector2D) (* (.A (Utilities|Struct|BreakLine (Utilities|Struct|MakeLine (Math|Vector2D|MakeVector2D (Math|Conversions|ToFloat(Integer) (.x (.a (.line _array_element)))) (Math|Conversions|ToFloat(Integer) (.y (.a (.line _array_element))))) (Math|Vector2D|MakeVector2D (Math|Conversions|ToFloat(Integer) (.x (.b (.line _array_element)))) (Math|Conversions|ToFloat(Integer) (.y (.b (.line _array_element)))))))) (Variables|Default|Getoffset2DVector))) "0.000000,90.000000,0.000000" "1.200000,1.000000,1.000000") true)
              (Components|InstancedStaticMesh|AddInstance _iemarch (Math|Transform|MakeTransform (Math|Conversions|ToVector(Vector2D) (* (.B (Utilities|Struct|BreakLine (Utilities|Struct|MakeLine (Math|Vector2D|MakeVector2D (Math|Conversions|ToFloat(Integer) (.x (.a (.line _array_element)))) (Math|Conversions|ToFloat(Integer) (.y (.a (.line _array_element))))) (Math|Vector2D|MakeVector2D (Math|Conversions|ToFloat(Integer) (.x (.b (.line _array_element)))) (Math|Conversions|ToFloat(Integer) (.y (.b (.line _array_element)))))))) (Variables|Default|Getoffset2DVector))) "0.000000,-90.000000,0.000000" "1.200000,1.000000,1.000000") true))))
        (:NewEnumerator1
          (Rendering|Debug|DrawDebugLine (Math|Conversions|ToVector(Vector2D) (* (.A (Utilities|Struct|BreakLine (Utilities|Struct|MakeLine (Math|Vector2D|MakeVector2D (Math|Conversions|ToFloat(Integer) (.x (.a (.line _array_element)))) (Math|Conversions|ToFloat(Integer) (.y (.a (.line _array_element))))) (Math|Vector2D|MakeVector2D (Math|Conversions|ToFloat(Integer) (.x (.b (.line _array_element)))) (Math|Conversions|ToFloat(Integer) (.y (.b (.line _array_element)))))))) (Variables|Default|Getoffset2DVector)) (Variables|Default|GetOffset%20Z)) (Math|Conversions|ToVector(Vector2D) (* (.B (Utilities|Struct|BreakLine (Utilities|Struct|MakeLine (Math|Vector2D|MakeVector2D (Math|Conversions|ToFloat(Integer) (.x (.a (.line _array_element)))) (Math|Conversions|ToFloat(Integer) (.y (.a (.line _array_element))))) (Math|Vector2D|MakeVector2D (Math|Conversions|ToFloat(Integer) (.x (.b (.line _array_element)))) (Math|Conversions|ToFloat(Integer) (.y (.b (.line _array_element)))))))) (Variables|Default|Getoffset2DVector)) (Variables|Default|GetOffset%20Z)) "(R=0.084274,G=0.199190,B=0.702083,A=1.000000)" 5e+03 3.0)
          (CallFunction|PlaceHallwayLineType (* (.A (Utilities|Struct|BreakLine (Utilities|Struct|MakeLine (Math|Vector2D|MakeVector2D (Math|Conversions|ToFloat(Integer) (.x (.a (.line _array_element)))) (Math|Conversions|ToFloat(Integer) (.y (.a (.line _array_element))))) (Math|Vector2D|MakeVector2D (Math|Conversions|ToFloat(Integer) (.x (.b (.line _array_element)))) (Math|Conversions|ToFloat(Integer) (.y (.b (.line _array_element)))))))) (Variables|Default|Getoffset2DVector)) (* (.B (Utilities|Struct|BreakLine (Utilities|Struct|MakeLine (Math|Vector2D|MakeVector2D (Math|Conversions|ToFloat(Integer) (.x (.a (.line _array_element)))) (Math|Conversions|ToFloat(Integer) (.y (.a (.line _array_element))))) (Math|Vector2D|MakeVector2D (Math|Conversions|ToFloat(Integer) (.x (.b (.line _array_element)))) (Math|Conversions|ToFloat(Integer) (.y (.b (.line _array_element)))))))) (Variables|Default|Getoffset2DVector))))
        (:NewEnumerator2
          (Rendering|Debug|DrawDebugLine (Math|Conversions|ToVector(Vector2D) (* (.A (Utilities|Struct|BreakLine (Utilities|Struct|MakeLine (Math|Vector2D|MakeVector2D (Math|Conversions|ToFloat(Integer) (.x (.a (.line _array_element)))) (Math|Conversions|ToFloat(Integer) (.y (.a (.line _array_element))))) (Math|Vector2D|MakeVector2D (Math|Conversions|ToFloat(Integer) (.x (.b (.line _array_element)))) (Math|Conversions|ToFloat(Integer) (.y (.b (.line _array_element)))))))) (Variables|Default|Getoffset2DVector)) (Variables|Default|GetOffset%20Z)) (Math|Conversions|ToVector(Vector2D) (* (.B (Utilities|Struct|BreakLine (Utilities|Struct|MakeLine (Math|Vector2D|MakeVector2D (Math|Conversions|ToFloat(Integer) (.x (.a (.line _array_element)))) (Math|Conversions|ToFloat(Integer) (.y (.a (.line _array_element))))) (Math|Vector2D|MakeVector2D (Math|Conversions|ToFloat(Integer) (.x (.b (.line _array_element)))) (Math|Conversions|ToFloat(Integer) (.y (.b (.line _array_element)))))))) (Variables|Default|Getoffset2DVector)) (Variables|Default|GetOffset%20Z)) "(R=0.000000,G=1.000000,B=0.958508,A=1.000000)" 5e+03 3.0))))
    (else
      (Utilities|String|LogString (.message GrpcResult)))))

(event EventBeginPlay
  (Variables|Default|SetOffset2DVector (Math|Vector2D|MakeVector2D (Math|Conversions|ToFloat(Integer) (Variables|Default|Getoffset)) (Math|Conversions|ToFloat(Integer) (Variables|Default|Getoffset))))
  (Variables|Default|SetOffset%20Z (Math|Conversions|ToFloat(Integer) (/ (Variables|Default|Getoffset) 2)))
  (Variables|Default|SetOffset%20Z (* (Variables|Default|GetOffset%20Z) 3.0))
  (Utilities|IsValid (Variables|Default|GetDungeonService)
    (:Is%20Not%20Valid
      (bind _returnvalue (Class|TurboLinkGrpcManager|MakeService (Subsystems|GetTurboLinkGrpcManager) "DungeonService"))
      (bind _asdungeon_service (Utilities|Casting|CastToDungeonService _returnvalue))
      (Variables|Default|SetDungeonService _asdungeon_service)
      (Class|DungeonService|Connect (Variables|Default|GetDungeonService))
      (bind _returnvalue_2 (Class|DungeonService|MakeClient (Variables|Default|GetDungeonService)))
      (bind _output_get (Variables|Default|SetDungeonServiceClient _returnvalue_2))
      (EventDispatchers|BindEventtoOnGenerateDungeonResponse _output_get (delegate Custom|OnGenerateDungeonResponse))
      (bind _returnvalue_3 (Class|DungeonServiceClient|InitGenerateDungeon (Variables|Default|GetDungeonServiceClient)))
      (Class|DungeonServiceClient|GenerateDungeon (Variables|Default|GetDungeonServiceClient) _returnvalue_3 (Utilities|Struct|MakeGrpcDungeonGenerateDungeonRequest 20 20 1000000 5 5) "(MetaData=())"))))

(event Collision|EventActorBeginOverlap
  (params (OtherActor :type Actor%20Object%20Reference)))

(event EventTick
  (params (DeltaSeconds :type Float%20%28single-precision%29)))

(fn ConstructionScript)

(fn GetOrientationfromTwoPoints
  (params (Vi :type Int%20Point%20Structure) (Vf :type Int%20Point%20Structure))
  (bind _vf (LocalVariables|Getvf))
  (bind _vf_2 (LocalVariables|Getvf))
  (bind _vi (LocalVariables|Getvi))
  (bind _vi_2 (LocalVariables|Getvi))
  (bind _vf_3 (LocalVariables|Getvf))
  (bind _vi_3 (LocalVariables|Getvi))
  (bind _vf_4 (LocalVariables|Getvf))
  (bind _vi_4 (LocalVariables|Getvi))
  (if (and (== (.x _vf) (.x _vi_2)) (> (.y _vf) (.y _vi_2)))
    (return "NewEnumerator1")
    (elif (and (< (.x _vf_3) (.x _vi_3)) (== (.y _vf_3) (.y _vi_3)))
      (return "NewEnumerator0")
      (elif (and (== (.x _vf_4) (.x _vi_4)) (< (.y _vf_4) (.y _vi_4)))
        (return "NewEnumerator1")
        (elif (and (> (.x _vf_2) (.x _vi)) (== (.y _vf_2) (.y _vi)))
          (return "NewEnumerator0"))))))

(fn PlaceHallwayLineType
  (params (vi :type Vector%202D%20Structure) (vf :type Vector%202D%20Structure))
  (LocalVariables|SettransformVector vi)
  (LocalVariables|Setdistance (/ (Math|Vector|Distance2D(Vector) vi vf) 2.0))
  (bind _horizontal (CallFunction|GetOrientationfromTwoPoints (Class|KismetMathLibrary|ToIntPoint(Vector2D) vi) (Class|KismetMathLibrary|ToIntPoint(Vector2D) vf)))
  (switch Utilities|FlowControl|Switch|SwitchonE_Orientation _horizontal
    (:NewEnumerator0
      (if (> (.x vi) (.x vf))
        (LocalVariables|SettransformVector vf))
      (Components|InstancedStaticMesh|AddInstance (Variables|Default|GetIEMWall) (Math|Transform|MakeTransform (Math|Vector|MakeVector (+ (.X (Math|Vector2D|BreakVector2D (LocalVariables|GettransformVector))) (LocalVariables|Getdistance)) (.Y (Math|Vector2D|BreakVector2D (LocalVariables|GettransformVector))) 0.0) "0, 0, 0" "0.750000,0.750000,1.000000") true))
    (:NewEnumerator1
      (if (> (.y vi) (.y vf))
        (LocalVariables|SettransformVector vf))
      (Components|InstancedStaticMesh|AddInstance (Variables|Default|GetIEMWall) (Math|Transform|MakeTransform (Math|Vector|MakeVector (.X (Math|Vector2D|BreakVector2D (LocalVariables|GettransformVector))) (+ (.Y (Math|Vector2D|BreakVector2D (LocalVariables|GettransformVector))) (LocalVariables|Getdistance)) 0.0) "0.000000,90.000000,0.000000" "0.750000,0.750000,1.000000") true))))