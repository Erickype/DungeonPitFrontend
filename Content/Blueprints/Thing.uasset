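; Blueprint that computes a 2D Delaunay triangulation from a point array using the Bowyer–Watson algorithm.
; It builds an enclosing super triangle, then inserts each point by removing triangles whose circumcircle contains it.
; Non-shared edges of removed triangles connect to the new point, and triangles touching super-triangle vertices are finally discarded.
; The EventGraph's call to the algorithm is unconnected, so nothing here runs it.
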(fn ConstructionScript)

(fn FindSuperTriangle
  (params (Points :type Array%20of%20Vector%202D%20Structures))
  (LocalVariables|SetMinX 1e+06)
  (LocalVariables|SetMinY 1e+06)
  (LocalVariables|SetMaxX -1e+06)
  (LocalVariables|SetMaxY -1e+06)
  (for _array_element Points
    (LocalVariables|SetMinX (Math|Float|Min(Float) (.x _array_element) (LocalVariables|GetMinX)))
    (LocalVariables|SetMinY (Math|Float|Min(Float) (.y _array_element) (LocalVariables|GetMinY)))
    (LocalVariables|SetMaxX (Math|Float|Max(Float) (.x _array_element) (LocalVariables|GetMaxX)))
    (LocalVariables|SetMaxY (Math|Float|Max(Float) (.y _array_element) (LocalVariables|GetMaxY))))
  (LocalVariables|Setdx (* (- (LocalVariables|GetMaxX) (LocalVariables|GetMinX)) 1.0))
  (LocalVariables|Setdy (* (- (LocalVariables|GetMaxY) (LocalVariables|GetMinY)) 1.0))
  (LocalVariables|SetdeltaMax (* (Math|Float|Max(Float) (LocalVariables|Getdx) (LocalVariables|Getdy)) 2.0))
  (return (Utilities|Struct|MakeTriangle (Math|Vector2D|MakeVector2D (- (LocalVariables|GetMinX) 1.0) (- (LocalVariables|GetMinY) 1.0)) (Math|Vector2D|MakeVector2D (- (LocalVariables|GetMinX) 1.0) (+ (LocalVariables|GetMaxY) (LocalVariables|GetdeltaMax))) (Math|Vector2D|MakeVector2D (+ (LocalVariables|GetMaxX) (LocalVariables|GetdeltaMax)) (- (LocalVariables|GetMinY) 1.0))) (Math|Vector2D|MakeVector2D (- (LocalVariables|GetMinX) (LocalVariables|Getdx)) (- (LocalVariables|GetMinY) (* (LocalVariables|Getdy) 3.0))) (Math|Vector2D|MakeVector2D (- (LocalVariables|GetMinX) (LocalVariables|Getdx)) (+ (LocalVariables|GetMaxY) (LocalVariables|Getdy))) (Math|Vector2D|MakeVector2D (+ (LocalVariables|GetMaxX) (* (LocalVariables|Getdx) 3.0)) (+ (LocalVariables|Getdy) (LocalVariables|GetMaxY)))))

(fn AddVertex
  (params (%20%20%20 :type Vector%202D%20Structure) (triangles :type Array%20of%20Triangle%20Structures))
  ;[0 0.6953 1] initialize
  (LocalVariables|SetVertex %20%20%20)
  (Utilities|Array|Clear (LocalVariables|GetnewTriangles))
  (Utilities|Array|Clear (LocalVariables|GetnewEdges))
  (for _array_element triangles
    (bind _is_ (CallFunction|IsinCircumcircle? (LocalVariables|GetVertex) _array_element))
    (if _is_ ; inCircumcircle?
      (Utilities|Array|Add (LocalVariables|GetnewEdges) (Utilities|Struct|MakeLine (.A (Utilities|Struct|BreakTriangle _array_element)) (.B (Utilities|Struct|BreakTriangle _array_element))))
      (Utilities|Array|Add (LocalVariables|GetnewEdges) (Utilities|Struct|MakeLine (.B (Utilities|Struct|BreakTriangle _array_element)) (.C (Utilities|Struct|BreakTriangle _array_element))))
      (Utilities|Array|Add (LocalVariables|GetnewEdges) (Utilities|Struct|MakeLine (.A (Utilities|Struct|BreakTriangle _array_element)) (.C (Utilities|Struct|BreakTriangle _array_element))))
      (else
        (Utilities|Array|Add (LocalVariables|GetnewTriangles) _array_element))))
  (Utilities|Array|Clear (LocalVariables|GetnewEdges2))
  (Utilities|Array|Clear (LocalVariables|GetnotFUniqueEdges))
  (for _array_element_2 (LocalVariables|GetnewEdges)
    (if (or (Utilities|Array|ContainsItem (LocalVariables|GetnewEdges2) _array_element_2) (Utilities|Array|ContainsItem (LocalVariables|GetnewEdges2) (Utilities|Struct|MakeLine (.B (Utilities|Struct|BreakLine _array_element_2)) (.A (Utilities|Struct|BreakLine _array_element_2)))))
      (Utilities|Array|Add (LocalVariables|GetnotFUniqueEdges) _array_element_2)
      (Utilities|Array|RemoveItem (LocalVariables|GetnewEdges2) (Utilities|Struct|MakeLine (.B (Utilities|Struct|BreakLine _array_element_2)) (.A (Utilities|Struct|BreakLine _array_element_2))))
      (Utilities|Array|RemoveItem (LocalVariables|GetnewEdges2) _array_element_2)
      (elif (not (or (Utilities|Array|ContainsItem (LocalVariables|GetnotFUniqueEdges) _array_element_2) (Utilities|Array|ContainsItem (LocalVariables|GetnotFUniqueEdges) (Utilities|Struct|MakeLine (.B (Utilities|Struct|BreakLine _array_element_2)) (.A (Utilities|Struct|BreakLine _array_element_2))))))
        (Utilities|Array|Add (LocalVariables|GetnewEdges2) _array_element_2))))
  (for _array_element_3 (LocalVariables|GetnewEdges2)
    (Utilities|Array|Add (LocalVariables|GetnewTriangles) (Utilities|Struct|MakeTriangle (.A (Utilities|Struct|BreakLine _array_element_3)) (.B (Utilities|Struct|BreakLine _array_element_3)) (LocalVariables|GetVertex))))
  (return (LocalVariables|GetnewTriangles)))

(fn Bowyer–WatsonAlgorithm
  (params (Points :type Array%20of%20Vector%202D%20Structures))
  (LocalVariables|SetPoints2 Points)
  (bind _triangle (CallFunction|FindSuperTriangle (LocalVariables|GetPoints2)))
  (bind _output_get (LocalVariables|SetSuperTriangle2 _triangle))
  (LocalVariables|SetTriangles%202 (Utilities|Array|MakeArray _output_get))
  (for _array_element (LocalVariables|GetPoints2)
    (bind _triangles_ (CallFunction|AddVertex _array_element (LocalVariables|GetTriangles%202)))
    (LocalVariables|SetTriangles%202 _triangles_))
  (for _array_element_2 (LocalVariables|GetTriangles%202)
    (if (not (Math|Boolean|ORBoolean (Class|KismetMathLibrary|EqualExactlyVector2DVector2D (.A (Utilities|Struct|BreakTriangle _array_element_2)) (.A (Utilities|Struct|BreakTriangle (LocalVariables|GetSuperTriangle2)))) (Class|KismetMathLibrary|EqualExactlyVector2DVector2D (.A (Utilities|Struct|BreakTriangle _array_element_2)) (.B (Utilities|Struct|BreakTriangle (LocalVariables|GetSuperTriangle2)))) (Class|KismetMathLibrary|EqualExactlyVector2DVector2D (.A (Utilities|Struct|BreakTriangle _array_element_2)) (.C (Utilities|Struct|BreakTriangle (LocalVariables|GetSuperTriangle2)))) (Class|KismetMathLibrary|EqualExactlyVector2DVector2D (.B (Utilities|Struct|BreakTriangle _array_element_2)) (.A (Utilities|Struct|BreakTriangle (LocalVariables|GetSuperTriangle2)))) (Class|KismetMathLibrary|EqualExactlyVector2DVector2D (.B (Utilities|Struct|BreakTriangle _array_element_2)) (.B (Utilities|Struct|BreakTriangle (LocalVariables|GetSuperTriangle2)))) (Class|KismetMathLibrary|EqualExactlyVector2DVector2D (.B (Utilities|Struct|BreakTriangle _array_element_2)) (.C (Utilities|Struct|BreakTriangle (LocalVariables|GetSuperTriangle2)))) (Class|KismetMathLibrary|EqualExactlyVector2DVector2D (.C (Utilities|Struct|BreakTriangle _array_element_2)) (.A (Utilities|Struct|BreakTriangle (LocalVariables|GetSuperTriangle2)))) (Class|KismetMathLibrary|EqualExactlyVector2DVector2D (.C (Utilities|Struct|BreakTriangle _array_element_2)) (.B (Utilities|Struct|BreakTriangle (LocalVariables|GetSuperTriangle2)))) (Class|KismetMathLibrary|EqualExactlyVector2DVector2D (.C (Utilities|Struct|BreakTriangle _array_element_2)) (.C (Utilities|Struct|BreakTriangle (LocalVariables|GetSuperTriangle2))))))
      (Utilities|Array|Add (LocalVariables|GetNewTriangles2) _array_element_2)))
  (return (LocalVariables|GetNewTriangles2)))

(fn IsinCircumcircle?
  (params (vertex :type Vector%202D%20Structure) (triangle :type Triangle%20Structure) (trinagle%20A :type Vector%202D%20Structure) (triangle%20B :type Vector%202D%20Structure) (triangle%20C :type Vector%202D%20Structure))
  (bind (_a _b _c) (Utilities|Struct|BreakTriangle triangle))
  (bind (_x _y) (Math|Vector2D|BreakVector2D _a))
  (bind (_x_2 _y_2) (Math|Vector2D|BreakVector2D _c))
  (bind (_x_3 _y_3) (Math|Vector2D|BreakVector2D _b))
  (LocalVariables|SetVertex%20X (.x vertex))
  (LocalVariables|SetVertex%20Y (.y vertex))
  (LocalVariables|Setax _x)
  (LocalVariables|Setay _y)
  (LocalVariables|Setbx _x_3)
  (LocalVariables|Setby _y_3)
  (LocalVariables|Setcx _x_2)
  (LocalVariables|Setcy _y_2)
  (LocalVariables|SetD (+ (* (LocalVariables|Getax) (- (LocalVariables|Getby) (LocalVariables|Getcy))) (* (LocalVariables|Getbx) (- (LocalVariables|Getcy) (LocalVariables|Getay))) (* (LocalVariables|Getcx) (- (LocalVariables|Getay) (LocalVariables|Getby)))))
  (LocalVariables|Setux (Utilities|Operators|Divide (+ (* (+ (Math|Float|Square (LocalVariables|Getax)) (Math|Float|Square (LocalVariables|Getay))) (- (LocalVariables|Getby) (LocalVariables|Getcy))) (* (+ (Math|Float|Square (LocalVariables|Getbx)) (Math|Float|Square (LocalVariables|Getby))) (- (LocalVariables|Getcy) (LocalVariables|Getay))) (* (+ (Math|Float|Square (LocalVariables|Getcx)) (Math|Float|Square (LocalVariables|Getcy))) (- (LocalVariables|Getay) (LocalVariables|Getby)))) (LocalVariables|GetD) 2.0))
  (LocalVariables|Setuy (Utilities|Operators|Divide (+ (* (+ (Math|Float|Square (LocalVariables|Getax)) (Math|Float|Square (LocalVariables|Getay))) (- (LocalVariables|Getcx) (LocalVariables|Getbx))) (* (+ (Math|Float|Square (LocalVariables|Getbx)) (Math|Float|Square (LocalVariables|Getby))) (- (LocalVariables|Getax) (LocalVariables|Getcx))) (* (+ (Math|Float|Square (LocalVariables|Getcx)) (Math|Float|Square (LocalVariables|Getcy))) (- (LocalVariables|Getbx) (LocalVariables|Getax)))) (LocalVariables|GetD) 2.0))
  (return (<= (Math|Vector2D|Vector2DLength (Math|Vector2D|MakeVector2D (- (LocalVariables|Getux) (LocalVariables|GetVertex%20X)) (- (LocalVariables|Getuy) (LocalVariables|GetVertex%20Y)))) (Math|Vector|Distance2D(Vector) (Math|Vector2D|MakeVector2D (LocalVariables|Getax) (LocalVariables|Getay)) (Math|Vector2D|MakeVector2D (LocalVariables|Getux) (LocalVariables|Getuy))))))