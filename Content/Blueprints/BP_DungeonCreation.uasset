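; BP_DungeonCreation is an actor that fetches dungeon data from a gRPC server and builds the room layout at runtime.
; On BeginPlay it connects a TurboLink DungeonService client and logs in with Username, then requests dungeon data using the returned player ID.
; Each room becomes an instanced static mesh, with axes remapped, offset by the last room's absolute Y and scaled by RoomsOffset, plus a debug coordinate label.
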(event Custom|OnGetDungeonDataResponse
  (params (Handle :type Grpc%20Context%20Handle%20Structure) (GrpcResult :type Grpc%20Result%20Structure%20%28by%20ref%29) (Response :type Grpc%20Game%20Get%20Dungeon%20Data%20Response%20Structure%20%28by%20ref%29))
  (bind (_code _message) (Utilities|Struct|BreakGrpcResult GrpcResult))
  (if (Utilities|Enum|Equal(Enum) _code "Ok")
    (bind _output_get (Variables|Default|SetRooms (Class|GrpcGameGetDungeonDataResponseHelperLibrary|BreakGetDungeonDataResponse Response)))
    (if (> (Utilities|Array|Length _output_get) 0)
      (bind _output_get_2 (Variables|Default|SetDungeonYOffset (Math|Integer|Absolute(Integer) (.Y (Utilities|Struct|BreakGrpcGameRoomResponse (Utilities|Array|Get(acopy) (Variables|Default|GetRooms) (Utilities|Array|LastIndex (Variables|Default|GetRooms))))))))
      (Utilities|String|LogString (Utilities|String|ToString(Integer) _output_get_2))
      (for _array_element (Variables|Default|GetRooms)
        (Components|InstancedStaticMesh|AddInstance (Variables|Default|GetInstancedStaticMesh) (Math|Transform|MakeTransform (Math|Vector|MakeVector (Math|Conversions|ToFloat(Integer) (* (+ (.X (Utilities|Struct|BreakGrpcGameRoomResponse _array_element)) (Variables|Default|GetDungeonYOffset)) (Variables|Default|GetRoomsOffset))) (Math|Conversions|ToFloat(Integer) (* (+ (* (.Z (Utilities|Struct|BreakGrpcGameRoomResponse _array_element)) -1) (Variables|Default|GetDungeonYOffset)) (Variables|Default|GetRoomsOffset))) (Math|Conversions|ToFloat(Integer) (* (+ (.Y (Utilities|Struct|BreakGrpcGameRoomResponse _array_element)) (Variables|Default|GetDungeonYOffset)) (Variables|Default|GetRoomsOffset))))) false)
        (Rendering|Debug|DrawDebugString (+ (Math|Vector|MakeVector (Math|Conversions|ToFloat(Integer) (* (+ (.X (Utilities|Struct|BreakGrpcGameRoomResponse _array_element)) (Variables|Default|GetDungeonYOffset)) (Variables|Default|GetRoomsOffset))) (Math|Conversions|ToFloat(Integer) (* (+ (* (.Z (Utilities|Struct|BreakGrpcGameRoomResponse _array_element)) -1) (Variables|Default|GetDungeonYOffset)) (Variables|Default|GetRoomsOffset))) (Math|Conversions|ToFloat(Integer) (* (+ (.Y (Utilities|Struct|BreakGrpcGameRoomResponse _array_element)) (Variables|Default|GetDungeonYOffset)) (Variables|Default|GetRoomsOffset)))) "0.000000,0.000000,50.000000") (Utilities|String|Append (Utilities|String|Append (Utilities|String|ToString(Integer) (.X (Utilities|Struct|BreakGrpcGameRoomResponse _array_element))) (Utilities|String|ToString(Integer) (.Y (Utilities|Struct|BreakGrpcGameRoomResponse _array_element)))) (Utilities|String|ToString(Integer) (.Z (Utilities|Struct|BreakGrpcGameRoomResponse _array_element)))) 0 "(R=0.000000,G=0.000000,B=0.000000,A=1.000000)" 5e+03))
      (else
        (Development|PrintText "Empty array runtime")))
    (else
      (Utilities|String|LogString _message))))

(event Custom|OnLoginResponse
  (params (Handle :type Grpc%20Context%20Handle%20Structure) (GrpcResult :type Grpc%20Result%20Structure%20%28by%20ref%29) (Response :type Grpc%20Game%20Login%20Response%20Structure%20%28by%20ref%29))
  (bind (_code _message) (Utilities|Struct|BreakGrpcResult GrpcResult))
  (bind _dungeonserviceclient (Variables|Default|GetDungeonServiceClient))
  (if (Utilities|Enum|Equal(Enum) _code "Ok")
    (bind _output_get (Variables|Default|SetPlayer%20Id (Utilities|Struct|BreakGrpcGameLoginResponse Response)))
    (Variables|Default|SetPlayerLogged true)
    (Utilities|String|LogString _output_get)
    (EventDispatchers|BindEventtoOnGetDungeonDataResponse (Variables|Default|GetDungeonServiceClient) (delegate Custom|OnGetDungeonDataResponse))
    (bind _returnvalue (Class|DungeonServiceClient|InitGetDungeonData _dungeonserviceclient))
    (Class|DungeonServiceClient|GetDungeonData _dungeonserviceclient _returnvalue (Utilities|Struct|MakeGrpcGameGetDungeonDataRequest (Variables|Default|GetPlayer%20Id)) "(MetaData=())")
    (else
      (Utilities|String|LogString _message))))

(event EventBeginPlay
  (Utilities|IsValid (Variables|Default|GetDungeonService)
    (:Is%20Not%20Valid
      (bind _returnvalue (Class|TurboLinkGrpcManager|MakeService (Subsystems|GetTurboLinkGrpcManager) "DungeonService"))
      (bind _asdungeon_service (Utilities|Casting|CastToDungeonService _returnvalue))
      (Variables|Default|SetDungeonService _asdungeon_service)
      (Class|DungeonService|Connect (Variables|Default|GetDungeonService))
      (bind _returnvalue_2 (Class|DungeonService|MakeClient (Variables|Default|GetDungeonService)))
      (bind _output_get (Variables|Default|SetDungeonServiceClient _returnvalue_2))
      (EventDispatchers|BindEventtoOnLoginResponse _output_get (delegate Custom|OnLoginResponse))
      (bind _returnvalue_3 (Class|DungeonServiceClient|InitLogin (Variables|Default|GetDungeonServiceClient)))
      (Class|DungeonServiceClient|Login (Variables|Default|GetDungeonServiceClient) _returnvalue_3 (Utilities|Struct|MakeGrpcGameLoginRequest (Variables|Default|GetUsername)) "(MetaData=())"))))

(event Collision|EventActorBeginOverlap
  (params (OtherActor :type Actor%20Object%20Reference)))

(event EventTick
  (params (DeltaSeconds :type Float%20%28single-precision%29)))

(fn ConstructionScript)